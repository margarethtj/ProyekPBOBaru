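; BP_Ball is one ball in a marble-chain style row that travels along a spline owned by SplineParent.
; Each tick it steps IndexLocation by Move and sweeps to that spline distance scaled by Space, with balls staggered by Index.
; Backward movement flips forward after CountBall × Target ticks.
; A free ball overlapping it inherits its spline data, stops simulating physics, and SplineParent halts, inserts and re-indexes the chain.
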(event OnComponentBeginOverlap(Bola)
  (params (OverlappedComponent :type Primitive%20Component%20Object%20Reference) (OtherActor :type Actor%20Object%20Reference) (OtherComp :type Primitive%20Component%20Object%20Reference) (OtherBodyIndex :type Integer) (bFromSweep :type Boolean) (SweepResult :type Hit%20Result%20Structure%20%28by%20ref%29))
  (bind _asbp_ball (Utilities|Casting|CastToBP_Ball OtherActor))
  (if (not (Variables|BP_Ball_C|GetisinSpline? _asbp_ball))
    (CallFunction|SetNewBallinfo _asbp_ball)
    (Physics|SetSimulatePhysics (Variables|BP_Ball_C|GetBola _asbp_ball) false)
    (Default|StopAllBall (Variables|Default|GetsplineParent))
    (if (== (Variables|Default|GetIndex) 0)
      (Default|InsertBall (Variables|Default|GetsplineParent) (Variables|Default|GetIndex) _asbp_ball)
      (Default|ResetIndex (Variables|Default|GetsplineParent))
      (else
        ;[1 1 1] fungsi dibalik index location keganti karena async function
        (Default|InsertBall (Variables|Default|GetsplineParent) (Variables|Default|GetIndex) _asbp_ball)
        (Default|ShiftBall (Variables|Default|GetsplineParent) (Variables|Default|GetIndex) (Variables|Default|GetIndexLocation))
        (Default|ResetIndex (Variables|Default|GetsplineParent))))))

(event Custom|get_index_frame
  (params (Space :type Float%20%28double-precision%29))
  (Variables|Default|SetSpace Space))

(event Custom|MovingAgain
  (Variables|Default|Setistick? true)
  (Variables|Default|SetisinSpline? true)
  (Variables|Default|SetisMoving? true))

(event Custom|SetNewBallinfo
  (params (NewBall :type BP%20Ball%20Object%20Reference))
  (CallFunction|GetIndexFrame NewBall (Variables|Default|GetSpace))
  (Variables|BP_Ball_C|SetisinSpline? NewBall true)
  (bind _output_get (Variables|BP_Ball_C|SetIndex NewBall (Variables|Default|GetIndex)))
  (Variables|BP_Ball_C|SetSpline%20Ref NewBall (Variables|Default|GetSpline%20Ref))
  (Variables|BP_Ball_C|SetsplineParent NewBall (Variables|Default|GetsplineParent))
  (if (== _output_get 0)
    (Variables|BP_Ball_C|SetIndexLocation NewBall (+ (Variables|Default|GetIndexLocation) 90))
    (else
      (Variables|BP_Ball_C|SetIndexLocation NewBall (Variables|Default|GetIndexLocation)))))

(event Custom|get_count
  (params (count :type Integer) (move :type Integer))
  (Variables|Default|SetCountBall count)
  (Variables|Default|SetMove move))

(event EventBeginPlay
  (Variables|Default|SetIndexLocation (+ (Variables|Default|GetIndexLocation) (* -90 (Variables|Default|GetIndex))))
  (Variables|Default|SetisMoving? true))

(event EventTick
  (params (DeltaSeconds :type Float%20%28single-precision%29))
  (if (Math|Boolean|ANDBoolean (Variables|Default|GetisMoving?) (Variables|Default|GetisinSpline?) (Variables|Default|Getistick?))
    (Utilities|FlowControl|Sequence
      (:then_0
        (bind _output_get (Variables|Default|SetIndexLocation (+ (Variables|Default|GetIndexLocation) (Variables|Default|GetMove))))
        (if (== (Variables|Default|GetMove) -1)
          (bind _result (Math|Integer|IncrementInt (Variables|Default|GetcounterTotal))
            (:%20%20
              (if (== (* (Variables|Default|GetCountBall) (Variables|Default|Gettarget)) _result)
                (Variables|Default|SetMove 1)
                (Variables|Default|SetcounterTotal 0)
                (Variables|/Game/Map/BP_RoadSpline.BP_RoadSpline_C|SetisBackward? (Variables|Default|GetsplineParent) false))))))
      (:then_1
        (if (not (< _output_get 0))
          (Transformation|SetActorLocation (Spline|GetLocationatDistanceAlongSpline (Variables|Default|GetSpline%20Ref) (* _output_get (Variables|Default|GetSpace)) "World") true true))))))

(fn ConstructionScript)