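; Cat Blueprint that spawns colored and special balls and plays a shooting animation, apparently as the shooter in a ball game.
; SpawnBall switches on an index to spawn one of nine ball classes at a fixed location, stores it in BPBall, clears Istick and disables its collision.
; The index is hardcoded to red, leaving the random roll unused.
; Shoot only plays the montage; BeginPlay and Coba are empty.
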(event Custom|Shoot
  (Animation|Montage|PlayMontage (Variables|Character|GetMesh) "/Game/Assets/Shooter/Montage_Shoot.Montage_Shoot"))

(event Custom|Spawn%20Ball
  (bind _output_get (Variables|Default|Setrandom 0))
  (switch int _output_get
    (:0
      (bind _returnvalue (Game|SpawnActorfromClass "/Game/Blueprint/BP_RedBall.BP_RedBall_C" (Math|Transform|MakeTransform "-375.000000,135.000000,50.000000" "0, 0, 0" "1.000000,1.000000,1.000000") "Undefined" 0 0 0 false 0 45 90 0))
      (bind _output_get_2 (Variables|Default|SetBP_Ball _returnvalue))
      (Variables|/Game/Blueprint/BP_Ball.BP_Ball_C|Setistick? _output_get_2 false)
      (Collision|SetCollisionEnabled (Variables|/Game/Blueprint/BP_Ball.BP_Ball_C|GetBola _output_get_2) "NoCollision"))
    (:1
      (bind _returnvalue_2 (Game|SpawnActorfromClass "/Game/Blueprint/BP_OrangeBall.BP_OrangeBall_C" (Math|Transform|MakeTransform "-375.000000,135.000000,50.000000" "0, 0, 0" "1.000000,1.000000,1.000000") "Undefined" 0 0 0 false 0 45 90 0))
      (bind _output_get_3 (Variables|Default|SetBP_Ball _returnvalue_2))
      (Variables|/Game/Blueprint/BP_Ball.BP_Ball_C|Setistick? _output_get_3 false)
      (Collision|SetCollisionEnabled (Variables|/Game/Blueprint/BP_Ball.BP_Ball_C|GetBola _output_get_3) "NoCollision"))
    (:2
      (bind _returnvalue_3 (Game|SpawnActorfromClass "/Game/Blueprint/BP_YellowBall.BP_YellowBall_C" (Math|Transform|MakeTransform "-375.000000,135.000000,50.000000" "0, 0, 0" "1.000000,1.000000,1.000000") "Undefined" 0 0 0 false 0 45 90 0))
      (bind _output_get_4 (Variables|Default|SetBP_Ball _returnvalue_3))
      (Variables|/Game/Blueprint/BP_Ball.BP_Ball_C|Setistick? _output_get_4 false)
      (Collision|SetCollisionEnabled (Variables|/Game/Blueprint/BP_Ball.BP_Ball_C|GetBola _output_get_4) "NoCollision"))
    (:3
      (bind _returnvalue_4 (Game|SpawnActorfromClass "/Game/Blueprint/BP_GreenBall.BP_GreenBall_C" (Math|Transform|MakeTransform "-375.000000,135.000000,50.000000" "0, 0, 0" "1.000000,1.000000,1.000000") "Undefined" 0 0 0 false 0 45 90 0))
      (bind _output_get_5 (Variables|Default|SetBP_Ball _returnvalue_4))
      (Variables|/Game/Blueprint/BP_Ball.BP_Ball_C|Setistick? _output_get_5 false)
      (Collision|SetCollisionEnabled (Variables|/Game/Blueprint/BP_Ball.BP_Ball_C|GetBola _output_get_5) "NoCollision"))
    (:4
      (bind _returnvalue_5 (Game|SpawnActorfromClass "/Game/Blueprint/BP_BlueBall.BP_BlueBall_C" (Math|Transform|MakeTransform "-375.000000,135.000000,50.000000" "0, 0, 0" "1.000000,1.000000,1.000000") "Undefined" 0 0 0 false 0 45 90 0))
      (bind _output_get_6 (Variables|Default|SetBP_Ball _returnvalue_5))
      (Variables|/Game/Blueprint/BP_Ball.BP_Ball_C|Setistick? _output_get_6 false)
      (Collision|SetCollisionEnabled (Variables|/Game/Blueprint/BP_Ball.BP_Ball_C|GetBola _output_get_6) "NoCollision"))
    (:5
      (bind _returnvalue_6 (Game|SpawnActorfromClass "/Game/Blueprint/BP_PinkBall.BP_PinkBall_C" (Math|Transform|MakeTransform "-375.000000,135.000000,50.000000" "0, 0, 0" "1.000000,1.000000,1.000000") "Undefined" 0 0 0 false 0 45 90 0))
      (bind _output_get_7 (Variables|Default|SetBP_Ball _returnvalue_6))
      (Variables|/Game/Blueprint/BP_Ball.BP_Ball_C|Setistick? _output_get_7 false)
      (Collision|SetCollisionEnabled (Variables|/Game/Blueprint/BP_Ball.BP_Ball_C|GetBola _output_get_7) "NoCollision"))
    (:6
      (bind _returnvalue_7 (Game|SpawnActorfromClass "/Game/Blueprint/BP_PurpleBall.BP_PurpleBall_C" (Math|Transform|MakeTransform "-375.000000,135.000000,50.000000" "0, 0, 0" "1.000000,1.000000,1.000000") "Undefined" 0 0 0 false 0 45 90 0))
      (bind _output_get_8 (Variables|Default|SetBP_Ball _returnvalue_7))
      (Variables|/Game/Blueprint/BP_Ball.BP_Ball_C|Setistick? _output_get_8 false)
      (Collision|SetCollisionEnabled (Variables|/Game/Blueprint/BP_Ball.BP_Ball_C|GetBola _output_get_8) "NoCollision"))
    (:7
      (bind _returnvalue_8 (Game|SpawnActorfromClass "/Game/Blueprint/BP_FireBall.BP_FireBall_C" (Math|Transform|MakeTransform "-375.000000,135.000000,50.000000" "0, 0, 0" "1.000000,1.000000,1.000000") "Undefined" 0 0 0 false 0 45 90 0))
      (bind _output_get_9 (Variables|Default|SetBP_Ball _returnvalue_8))
      (Variables|/Game/Blueprint/BP_Ball.BP_Ball_C|Setistick? _output_get_9 false)
      (Collision|SetCollisionEnabled (Variables|/Game/Blueprint/BP_Ball.BP_Ball_C|GetBola _output_get_9) "NoCollision"))
    (:8
      (bind _returnvalue_9 (Game|SpawnActorfromClass "/Game/Blueprint/BP_IceBall.BP_IceBall_C" (Math|Transform|MakeTransform "-375.000000,135.000000,50.000000" "0, 0, 0" "1.000000,1.000000,1.000000") "Undefined" 0 0 0 false 0 45 90 0))
      (bind _output_get_10 (Variables|Default|SetBP_Ball _returnvalue_9))
      (Variables|/Game/Blueprint/BP_Ball.BP_Ball_C|Setistick? _output_get_10 false)
      (Collision|SetCollisionEnabled (Variables|/Game/Blueprint/BP_Ball.BP_Ball_C|GetBola _output_get_10) "NoCollision"))))

(event EventBeginPlay)

(fn ConstructionScript)

(fn Coba)