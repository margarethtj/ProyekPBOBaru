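; BP_GameModeZuma is a game mode that tracks elapsed time and score, and shows a Timer widget at BeginPlay.
; Tick counts seconds into minutes continuously, independent of StartTimer.
; E calls StartTimer, which only sets a zero-length, non-looping timer targeting itself, while F calls TimerReset to clear that handle and zero the clock.
; AddScore adds the passed value to Score.
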(event Custom|AddScore
  (params (TotalScore :type Integer))
  (Variables|Default|SetScore (+ TotalScore (Variables|Default|GetScore))))

(event Custom|Start%20Timer
  (bind _returnvalue (Utilities|Time|SetTimerbyEvent (delegate Custom|Start%20Timer) 0.0)))

(event Custom|Timer%20Reset
  (Utilities|Time|ClearandInvalidateTimerbyHandle (stale Custom|Start%20Timer _returnvalue))
  (Variables|Default|SetTimerSeconds 0.0)
  (Variables|Default|SetTimerMinutes 0.0))

(event EventBeginPlay
  (bind _returnvalue (UserInterface|CreateWidget "/Game/Blueprint/UI/Timer.Timer_C"))
  (UserInterface|Viewport|AddtoViewport _returnvalue 0))

(event EventTick
  (params (DeltaSeconds :type Float%20%28single-precision%29))
  (Variables|Default|SetTimerSeconds (+ (Variables|Default|GetTimerSeconds) DeltaSeconds))
  (if (>= (Variables|Default|GetTimerSeconds) 6e+01)
    (Variables|Default|SetTimerSeconds 0.0)
    (Variables|Default|SetTimerMinutes (+ (Variables|Default|GetTimerMinutes) 1.0))))

(event Input|KeyboardEvents|E
  (params (Key :type Key%20Structure :default "None"))
  (:Pressed
    (bind _asbp_game_mode_zuma (Utilities|Casting|CastToBP_GameModeZuma (Game|GetGameMode)))
    (CallFunction|StartTimer _asbp_game_mode_zuma)))

(event Input|KeyboardEvents|F
  (params (Key :type Key%20Structure :default "None"))
  (:Pressed
    (bind _asbp_game_mode_zuma (Utilities|Casting|CastToBP_GameModeZuma (Game|GetGameMode)))
    (CallFunction|TimerReset _asbp_game_mode_zuma)))

(fn ConstructionScript)