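; BP_OrangeBall is the orange ball Blueprint in what appears to be a Zuma-style game.
; Its GetScore event casts the game mode to BP_GameModeZuma and sets Score to 15, overwriting the value rather than adding to it.
; BeginPlay, overlap and Tick are disabled placeholder nodes, and the construction script only calls the parent.
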(event EventBeginPlay
  (|CallParentFunction) ; This node is disabled and will not be called.\nDrag off pins to build functionality.
)

(event Collision|EventActorBeginOverlap
  (params (OtherActor :type Actor%20Object%20Reference))
  (|CallParentFunction OtherActor) ; This node is disabled and will not be called.\nDrag off pins to build functionality.
)

(event EventTick
  (params (DeltaSeconds :type Float%20%28single-precision%29))
  (|CallParentFunction DeltaSeconds) ; This node is disabled and will not be called.\nDrag off pins to build functionality.
)

(event EventGetScore
  (bind _asbp_game_mode_zuma (Utilities|Casting|CastToBP_GameModeZuma (Game|GetGameMode)))
  (Variables|/Game/Blueprint/BP_GameModeZuma.BP_GameModeZuma_C|SetScore _asbp_game_mode_zuma 15))

(fn ConstructionScript
  (|CallParentFunction))