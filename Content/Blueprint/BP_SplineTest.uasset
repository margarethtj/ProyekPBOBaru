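; Test actor that populates a spline with child actors in its construction script, expected to be BP_BoxCollisionCustom.
; Spline length divided by 32 sets both the spacing and, truncated, the last loop index.
; Each child is placed at index times spacing along the spline in local space and receives that index through a cast.
; Event graph holds only disabled stub events.
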(event EventBeginPlay)

(event Collision|EventActorBeginOverlap
  (params (OtherActor :type Actor%20Object%20Reference)))

(event EventTick
  (params (DeltaSeconds :type Float%20%28single-precision%29)))

(fn ConstructionScript
  (bind _spline (Variables|Default|GetSpline))
  (bind _returnvalue (Spline|GetSplineLength _spline))
  (bind _returnvalue_2 (/ _returnvalue 32.0))
  (bind _output_get (LocalVariables|SetSpace _returnvalue_2))
  (for _index (range 0 (Math|Float|Truncate _returnvalue_2))
    (bind _returnvalue_3 (AddComponent|AddChildActorComponent false (Math|Transform|MakeTransform (Spline|GetLocationatDistanceAlongSpline _spline (* _index _output_get) "Local") "0, 0, 0" "1.000000,1.000000,1.000000")))
    (bind _asbp_box_collision_custom (Utilities|Casting|CastToBP_BoxCollisionCustom (Variables|/Script/Engine.ChildActorComponent|GetChildActor _returnvalue_3)))
    (Variables|/Game/Blueprint/BP_BoxCollisionCustom.BP_BoxCollisionCustom_C|SetIndex _asbp_box_collision_custom _index)))