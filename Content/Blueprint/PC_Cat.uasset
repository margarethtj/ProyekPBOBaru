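; Player controller for a ball shooter that aims a cat at the mouse cursor and fires randomly chosen balls.
; BeginPlay caches BP_Cat, adds the input mapping and spawns a waiting, collision-free ball from nine colored, fire and ice types.
; Tick yaws the cat toward the cursor hit and draws a debug line-trace laser.
; IA_Shoot waits briefly, launches the ball from the cat's arrow with a physics impulse, then spawns the next.
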(event Custom|Spawn%20Ball
  (bind _output_get (Variables|Default|Setrandom (Math|Random|RandomIntegerinRange 0 8)))
  (switch int _output_get
    (:0
      (bind _returnvalue (Game|SpawnActorfromClass "/Game/Blueprint/BP_RedBall.BP_RedBall_C" (Math|Transform|MakeTransform "-375.000000,135.000000,50.000000" "0, 0, 0" "1.000000,1.000000,1.000000") "Undefined" 0 0 0 false 0 45 90 0))
      (bind _output_get_2 (Variables|Default|SetBP_Ball _returnvalue))
      (Variables|/Game/Blueprint/BP_Ball.BP_Ball_C|Setistick? _output_get_2 false)
      (Collision|SetCollisionEnabled (Variables|/Game/Blueprint/BP_Ball.BP_Ball_C|GetBola _output_get_2) "NoCollision"))
    (:1
      (bind _returnvalue_2 (Game|SpawnActorfromClass "/Game/Blueprint/BP_OrangeBall.BP_OrangeBall_C" (Math|Transform|MakeTransform "-375.000000,135.000000,50.000000" "0, 0, 0" "1.000000,1.000000,1.000000") "Undefined" 0 0 0 false 0 45 90 0))
      (bind _output_get_3 (Variables|Default|SetBP_Ball _returnvalue_2))
      (Variables|/Game/Blueprint/BP_Ball.BP_Ball_C|Setistick? _output_get_3 false)
      (Collision|SetCollisionEnabled (Variables|/Game/Blueprint/BP_Ball.BP_Ball_C|GetBola _output_get_3) "NoCollision"))
    (:2
      (bind _returnvalue_3 (Game|SpawnActorfromClass "/Game/Blueprint/BP_YellowBall.BP_YellowBall_C" (Math|Transform|MakeTransform "-375.000000,135.000000,50.000000" "0, 0, 0" "1.000000,1.000000,1.000000") "Undefined" 0 0 0 false 0 45 90 0))
      (bind _output_get_4 (Variables|Default|SetBP_Ball _returnvalue_3))
      (Variables|/Game/Blueprint/BP_Ball.BP_Ball_C|Setistick? _output_get_4 false)
      (Collision|SetCollisionEnabled (Variables|/Game/Blueprint/BP_Ball.BP_Ball_C|GetBola _output_get_4) "NoCollision"))
    (:3
      (bind _returnvalue_4 (Game|SpawnActorfromClass "/Game/Blueprint/BP_GreenBall.BP_GreenBall_C" (Math|Transform|MakeTransform "-375.000000,135.000000,50.000000" "0, 0, 0" "1.000000,1.000000,1.000000") "Undefined" 0 0 0 false 0 45 90 0))
      (bind _output_get_5 (Variables|Default|SetBP_Ball _returnvalue_4))
      (Variables|/Game/Blueprint/BP_Ball.BP_Ball_C|Setistick? _output_get_5 false)
      (Collision|SetCollisionEnabled (Variables|/Game/Blueprint/BP_Ball.BP_Ball_C|GetBola _output_get_5) "NoCollision"))
    (:4
      (bind _returnvalue_5 (Game|SpawnActorfromClass "/Game/Blueprint/BP_BlueBall.BP_BlueBall_C" (Math|Transform|MakeTransform "-375.000000,135.000000,50.000000" "0, 0, 0" "1.000000,1.000000,1.000000") "Undefined" 0 0 0 false 0 45 90 0))
      (bind _output_get_6 (Variables|Default|SetBP_Ball _returnvalue_5))
      (Variables|/Game/Blueprint/BP_Ball.BP_Ball_C|Setistick? _output_get_6 false)
      (Collision|SetCollisionEnabled (Variables|/Game/Blueprint/BP_Ball.BP_Ball_C|GetBola _output_get_6) "NoCollision"))
    (:5
      (bind _returnvalue_6 (Game|SpawnActorfromClass "/Game/Blueprint/BP_PinkBall.BP_PinkBall_C" (Math|Transform|MakeTransform "-375.000000,135.000000,50.000000" "0, 0, 0" "1.000000,1.000000,1.000000") "Undefined" 0 0 0 false 0 45 90 0))
      (bind _output_get_7 (Variables|Default|SetBP_Ball _returnvalue_6))
      (Variables|/Game/Blueprint/BP_Ball.BP_Ball_C|Setistick? _output_get_7 false)
      (Collision|SetCollisionEnabled (Variables|/Game/Blueprint/BP_Ball.BP_Ball_C|GetBola _output_get_7) "NoCollision"))
    (:6
      (bind _returnvalue_7 (Game|SpawnActorfromClass "/Game/Blueprint/BP_PurpleBall.BP_PurpleBall_C" (Math|Transform|MakeTransform "-375.000000,135.000000,50.000000" "0, 0, 0" "1.000000,1.000000,1.000000") "Undefined" 0 0 0 false 0 45 90 0))
      (bind _output_get_8 (Variables|Default|SetBP_Ball _returnvalue_7))
      (Variables|/Game/Blueprint/BP_Ball.BP_Ball_C|Setistick? _output_get_8 false)
      (Collision|SetCollisionEnabled (Variables|/Game/Blueprint/BP_Ball.BP_Ball_C|GetBola _output_get_8) "NoCollision"))
    (:7
      (bind _returnvalue_8 (Game|SpawnActorfromClass "/Game/Blueprint/BP_FireBall.BP_FireBall_C" (Math|Transform|MakeTransform "-375.000000,135.000000,50.000000" "0, 0, 0" "1.000000,1.000000,1.000000") "Undefined" 0 0 0 false 0 45 90 0))
      (bind _output_get_9 (Variables|Default|SetBP_Ball _returnvalue_8))
      (Variables|/Game/Blueprint/BP_Ball.BP_Ball_C|Setistick? _output_get_9 false)
      (Collision|SetCollisionEnabled (Variables|/Game/Blueprint/BP_Ball.BP_Ball_C|GetBola _output_get_9) "NoCollision"))
    (:8
      (bind _returnvalue_9 (Game|SpawnActorfromClass "/Game/Blueprint/BP_IceBall.BP_IceBall_C" (Math|Transform|MakeTransform "-375.000000,135.000000,50.000000" "0, 0, 0" "1.000000,1.000000,1.000000") "Undefined" 0 0 0 false 0 45 90 0))
      (bind _output_get_10 (Variables|Default|SetBP_Ball _returnvalue_9))
      (Variables|/Game/Blueprint/BP_Ball.BP_Ball_C|Setistick? _output_get_10 false)
      (Collision|SetCollisionEnabled (Variables|/Game/Blueprint/BP_Ball.BP_Ball_C|GetBola _output_get_10) "NoCollision"))))

(event Input|EnhancedActionEvents|EnhancedInputActionIA_Shoot
  (params (ActionValue :type Boolean) (ElapsedSeconds :type Float%20%28double-precision%29) (TriggeredSeconds :type Float%20%28double-precision%29) (InputAction :type Input%20Action%20Object%20Reference :default "/Game/Input/IA_Shoot.IA_Shoot"))
  (bind _bp_cat (Variables|Default|GetBp_Cat))
  (bind _bp_ball (Variables|Default|GetBP_Ball))
  (bind _arrow1 (Variables|/Game/Blueprint/BP_Cat.BP_Cat_C|GetArrow1 _bp_cat))
  (bind _bola (Variables|/Game/Blueprint/BP_Ball.BP_Ball_C|GetBola _bp_ball))
  (:Started
    (Utilities|FlowControl|Delay 0.5)
    (Transformation|SetActorLocation _bp_ball (Transformation|GetWorldLocation _arrow1) false true)
    (Collision|SetCollisionEnabled _bola "QueryAndPhysics")
    (Physics|SetSimulatePhysics _bola true)
    (Physics|AddImpulse _bola (* (Math|Vector|GetForwardVector _arrow1) 2.5e+03) "None" true)
    (CallFunction|SpawnBall)))

(event EventTick
  (params (DeltaSeconds :type Float%20%28single-precision%29))
  ;[0.401 0.401 0.401] LaserSystem
  (Transformation|SetActorRotation (Variables|Default|GetBp_Cat) (Math|Rotator|MakeRotator 0.0 0.0 (.yaw (Math|Rotator|FindLookatRotation (Transformation|GetActorLocation (Variables|Default|GetBp_Cat)) (.ImpactPoint (Collision|BreakHitResult (.HitResult (Game|Player|GetHitResultUnderCursorbyChannel "TraceTypeQuery1" true))))))))
  (CallFunction|LaserFunction))

(event EventBeginPlay
  (Utilities|FlowControl|Sequence
    (:then_0
      (Variables|Default|SetbShowMouseCursor true)
      (bind _outactors (Actor|GetAllActorsOfClass "/Game/Blueprint/BP_Cat.BP_Cat_C"))
      (Variables|Default|SetBp_Cat (Utilities|Array|Get(acopy) _outactors))
      (Input|AddMappingContext (PlayerController|LocalPlayerSubsystems|GetEnhancedInputLocalPlayerSubsystem) "/Game/Input/IMC_ContextMapping.IMC_ContextMapping" 0 "(bIgnoreAllPressedKeysUntilRelease=True,bForceImmediately=False)")
      (CallFunction|SpawnBall))))

(fn ConstructionScript)

(fn LaserFunction
  (bind _bp_cat (Variables|Default|GetBp_Cat))
  (bind _arrow1 (Variables|/Game/Blueprint/BP_Cat.BP_Cat_C|GetArrow1 _bp_cat))
  (LocalVariables|SetLocation (Transformation|GetWorldLocation _arrow1))
  (LocalVariables|SetForward (Math|Vector|GetForwardVector _arrow1))
  (Collision|LineTraceByChannel (LocalVariables|GetLocation) (+ (* (LocalVariables|GetForward) 1e+04) (LocalVariables|GetLocation)) "TraceTypeQuery1" true 0 "ForDuration" true "(R=1.000000,G=0.000000,B=0.000000,A=1.000000)" "(R=0.000000,G=1.000000,B=0.000000,A=1.000000)" 0.1))