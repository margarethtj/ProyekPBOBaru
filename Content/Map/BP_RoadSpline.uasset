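; Spline road actor for a marble-chain match game, which spawns and manages a line of randomly colored balls along its spline.
; Construction script lays spline meshes along the road, and BeginPlay spawns the starting balls into an ordered array.
; Events shift and insert balls by spline distance, stop or resume them, and reindex.
; A looping CheckCombo timer casts neighbors by color class, destroys runs of three or more, and triggers backward movement.
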(event Custom|StopAllBall
  (for _array_element (Variables|Default|GetarrayBola)
    (Variables|/Game/Blueprint/BP_Ball.BP_Ball_C|Setistick? _array_element false)))

(event Custom|MovingAgain
  (for _array_element (Variables|Default|GetarrayBola)
    (Default|MovingAgain _array_element)))

(event Custom|ShiftBall
  (params (index :type Integer) (indexLocation :type Integer))
  (for _index (range 0 index)
    (bind _output_get (Variables|/Game/Blueprint/BP_Ball.BP_Ball_C|SetIndexLocation (Utilities|Array|Get(acopy) (Variables|Default|GetarrayBola) _index) (+ (Variables|/Game/Blueprint/BP_Ball.BP_Ball_C|GetIndexLocation (Utilities|Array|Get(acopy) (Variables|Default|GetarrayBola) _index)) 30)))
    (Transformation|SetActorLocation (Utilities|Array|Get(acopy) (Variables|Default|GetarrayBola) _index) (Spline|GetLocationatDistanceAlongSpline (Variables|Default|GetRoad) (* _output_get (Variables|/Game/Blueprint/BP_Ball.BP_Ball_C|GetSpace (Utilities|Array|Get(acopy) (Variables|Default|GetarrayBola) _index))) "World") true true)))

(event Custom|InsertBall
  (params (index :type Integer) (ball :type BP%20Ball%20Object%20Reference))
  (bind _road (Variables|Default|GetRoad))
  (bind _space (Variables|/Game/Blueprint/BP_Ball.BP_Ball_C|GetSpace ball))
  (bind _indexlocation (Variables|/Game/Blueprint/BP_Ball.BP_Ball_C|GetIndexLocation ball))
  (bind _returnvalue (* _indexlocation _space))
  (bind _returnvalue_2 (Spline|GetLocationatDistanceAlongSpline _road _returnvalue "World"))
  (Utilities|Array|Insert (Variables|Default|GetarrayBola) ball index)
  (Development|PrintString (Utilities|String|Append (Utilities|String|ToString(Integer) _indexlocation) "bb"))
  (Development|PrintString (Utilities|String|ToString(Vector) _returnvalue_2))
  (Transformation|SetActorLocation ball _returnvalue_2 true true))

(event Custom|ResetIndex
  (for (_array_element _array_index) (Variables|Default|GetarrayBola)
    (Variables|/Game/Blueprint/BP_Ball.BP_Ball_C|SetIndex _array_element _array_index))
  (CallFunction|MovingAgain))

(event Custom|CheckCombo
  (bind _arraybola (Variables|Default|GetarrayBola))
  (bind _arraybola_2 (Variables|Default|GetarrayBola))
  (bind _arraybola_3 (Variables|Default|GetarrayBola))
  (bind _arraybola_4 (Variables|Default|GetarrayBola))
  (bind _arraybola_5 (Variables|Default|GetarrayBola))
  (bind _arraybola_6 (Variables|Default|GetarrayBola))
  (bind _arraybola_7 (Variables|Default|GetarrayBola))
  (bind _arraybola_8 (Variables|Default|GetarrayBola))
  (bind (_array_element _array_index) (Utilities|Array|ForEachLoopwithBreak _arraybola_3 :!label _label)
    (:LoopBody
      (Variables|Default|SetArray%20Index _array_index)
      (if (not (== (Variables|Default|GetArray%20Index) (- (Utilities|Array|LastIndex _arraybola_3) 1)))
        (Utilities|Casting|CastToBP_RedBall _array_element
          (:then
            (Utilities|Casting|CastToBP_RedBall (Utilities|Array|Get(acopy) (Variables|Default|GetarrayBola) (+ (Variables|Default|GetArray%20Index) 1))
              (:then
                (bind _result (Math|Integer|IncrementInt (Variables|Default|Getcount))
                  (:%20%20
                    (Variables|Default|Setcount _result))))
              (:CastFailed
                (if (>= (Variables|Default|Getcount) 3)
                  (Variables|Default|SetArrayIndexStartDelete (- (Variables|Default|GetArray%20Index) (- (Variables|Default|Getcount) 1)))
                  (for _index (range 0 (- (Variables|Default|Getcount) 1))
                    (bind _output_get (Variables|Default|SetTempObject (Utilities|Array|Get(acopy) _arraybola_5 (Variables|Default|GetArrayIndexStartDelete))))
                    (Utilities|Array|RemoveIndex _arraybola_5 (Variables|Default|GetArrayIndexStartDelete))
                    (Actor|DestroyActor _output_get)
                    (CallFunction|ResetIndex)
                    (CallFunction|MoveBackward self))
                  (Variables|Default|Settarget (* (Variables|Default|Getcount) 30))
                  (Variables|Default|Setcount 1)
                  (goto _label Break)
                  (else
                    (Variables|Default|Setcount 1)
                    (if (== (Variables|Default|GetArray%20Index) (- (Utilities|Array|LastIndex (Variables|Default|GetarrayBola)) 1))
                      (Variables|Default|Setrepeat false)
                      (goto _label Break)))))))
          (:CastFailed
            (Utilities|Casting|CastToBP_OrangeBall _array_element
              (:then
                (Utilities|Casting|CastToBP_OrangeBall (Utilities|Array|Get(acopy) (Variables|Default|GetarrayBola) (+ (Variables|Default|GetArray%20Index) 1))
                  (:then
                    (bind _result_2 (Math|Integer|IncrementInt (Variables|Default|Getcount))
                      (:%20%20
                        (Variables|Default|Setcount _result_2))))
                  (:CastFailed
                    (if (>= (Variables|Default|Getcount) 3)
                      (Variables|Default|SetArrayIndexStartDelete (- (Variables|Default|GetArray%20Index) (- (Variables|Default|Getcount) 1)))
                      (for _index_2 (range 0 (- (Variables|Default|Getcount) 1))
                        (bind _output_get_2 (Variables|Default|SetTempObject (Utilities|Array|Get(acopy) _arraybola_6 (Variables|Default|GetArrayIndexStartDelete))))
                        (Utilities|Array|RemoveIndex _arraybola_6 (Variables|Default|GetArrayIndexStartDelete))
                        (Actor|DestroyActor _output_get_2)
                        (CallFunction|ResetIndex)
                        (CallFunction|MoveBackward self))
                      (Variables|Default|Settarget (* (Variables|Default|Getcount) 30))
                      (Variables|Default|Setcount 1)
                      (goto _label Break)
                      (else
                        (Variables|Default|Setcount 1)
                        (if (== (Variables|Default|GetArray%20Index) (- (Utilities|Array|LastIndex (Variables|Default|GetarrayBola)) 1))
                          (Variables|Default|Setrepeat false)
                          (goto _label Break)))))))
              (:CastFailed
                (Utilities|Casting|CastToBP_YellowBall _array_element
                  (:then
                    (Utilities|Casting|CastToBP_YellowBall (Utilities|Array|Get(acopy) (Variables|Default|GetarrayBola) (+ (Variables|Default|GetArray%20Index) 1))
                      (:then
                        (bind _result_3 (Math|Integer|IncrementInt (Variables|Default|Getcount))
                          (:%20%20
                            (Variables|Default|Setcount _result_3))))
                      (:CastFailed
                        (if (>= (Variables|Default|Getcount) 3)
                          (Variables|Default|SetArrayIndexStartDelete (- (Variables|Default|GetArray%20Index) (- (Variables|Default|Getcount) 1)))
                          (for _index_3 (range 0 (- (Variables|Default|Getcount) 1))
                            (bind _output_get_3 (Variables|Default|SetTempObject (Utilities|Array|Get(acopy) _arraybola_7 (Variables|Default|GetArrayIndexStartDelete))))
                            (Utilities|Array|RemoveIndex _arraybola_7 (Variables|Default|GetArrayIndexStartDelete))
                            (Actor|DestroyActor _output_get_3)
                            (CallFunction|ResetIndex)
                            (CallFunction|MoveBackward self))
                          (Variables|Default|Settarget (* (Variables|Default|Getcount) 30))
                          (Variables|Default|Setcount 1)
                          (goto _label Break)
                          (else
                            (Variables|Default|Setcount 1)
                            (if (== (Variables|Default|GetArray%20Index) (- (Utilities|Array|LastIndex (Variables|Default|GetarrayBola)) 1))
                              (Variables|Default|Setrepeat false)
                              (goto _label Break)))))))
                  (:CastFailed
                    (Utilities|Casting|CastToBP_GreenBall _array_element
                      (:then
                        (Utilities|Casting|CastToBP_GreenBall (Utilities|Array|Get(acopy) (Variables|Default|GetarrayBola) (+ (Variables|Default|GetArray%20Index) 1))
                          (:then
                            (bind _result_4 (Math|Integer|IncrementInt (Variables|Default|Getcount))
                              (:%20%20
                                (Variables|Default|Setcount _result_4))))
                          (:CastFailed
                            (if (>= (Variables|Default|Getcount) 3)
                              (Variables|Default|SetArrayIndexStartDelete (- (Variables|Default|GetArray%20Index) (- (Variables|Default|Getcount) 1)))
                              (for _index_4 (range 0 (- (Variables|Default|Getcount) 1))
                                (bind _output_get_4 (Variables|Default|SetTempObject (Utilities|Array|Get(acopy) _arraybola_8 (Variables|Default|GetArrayIndexStartDelete))))
                                (Utilities|Array|RemoveIndex _arraybola_8 (Variables|Default|GetArrayIndexStartDelete))
                                (Actor|DestroyActor _output_get_4)
                                (CallFunction|ResetIndex)
                                (CallFunction|MoveBackward self))
                              (Variables|Default|Settarget (* (Variables|Default|Getcount) 30))
                              (Variables|Default|Setcount 1)
                              (goto _label Break)
                              (else
                                (Variables|Default|Setcount 1)
                                (if (== (Variables|Default|GetArray%20Index) (- (Utilities|Array|LastIndex (Variables|Default|GetarrayBola)) 1))
                                  (Variables|Default|Setrepeat false)
                                  (goto _label Break)))))))
                      (:CastFailed
                        (Utilities|Casting|CastToBP_BlueBall _array_element
                          (:then
                            (Utilities|Casting|CastToBP_BlueBall (Utilities|Array|Get(acopy) (Variables|Default|GetarrayBola) (+ (Variables|Default|GetArray%20Index) 1))
                              (:then
                                (bind _result_5 (Math|Integer|IncrementInt (Variables|Default|Getcount))
                                  (:%20%20
                                    (Variables|Default|Setcount _result_5))))
                              (:CastFailed
                                (if (>= (Variables|Default|Getcount) 3)
                                  (Variables|Default|SetArrayIndexStartDelete (- (Variables|Default|GetArray%20Index) (- (Variables|Default|Getcount) 1)))
                                  (for _index_5 (range 0 (- (Variables|Default|Getcount) 1))
                                    (bind _output_get_5 (Variables|Default|SetTempObject (Utilities|Array|Get(acopy) _arraybola (Variables|Default|GetArrayIndexStartDelete))))
                                    (Utilities|Array|RemoveIndex _arraybola (Variables|Default|GetArrayIndexStartDelete))
                                    (Actor|DestroyActor _output_get_5)
                                    (CallFunction|ResetIndex)
                                    (CallFunction|MoveBackward self))
                                  (Variables|Default|Settarget (* (Variables|Default|Getcount) 30))
                                  (Variables|Default|Setcount 1)
                                  (goto _label Break)
                                  (else
                                    (Variables|Default|Setcount 1)
                                    (if (== (Variables|Default|GetArray%20Index) (- (Utilities|Array|LastIndex (Variables|Default|GetarrayBola)) 1))
                                      (Variables|Default|Setrepeat false)
                                      (goto _label Break)))))))
                          (:CastFailed
                            (Utilities|Casting|CastToBP_PinkBall _array_element
                              (:then
                                (Utilities|Casting|CastToBP_PinkBall (Utilities|Array|Get(acopy) (Variables|Default|GetarrayBola) (+ (Variables|Default|GetArray%20Index) 1))
                                  (:then
                                    (bind _result_6 (Math|Integer|IncrementInt (Variables|Default|Getcount))
                                      (:%20%20
                                        (Variables|Default|Setcount _result_6))))
                                  (:CastFailed
                                    (if (>= (Variables|Default|Getcount) 3)
                                      (Variables|Default|SetArrayIndexStartDelete (- (Variables|Default|GetArray%20Index) (- (Variables|Default|Getcount) 1)))
                                      (for _index_6 (range 0 (- (Variables|Default|Getcount) 1))
                                        (bind _output_get_6 (Variables|Default|SetTempObject (Utilities|Array|Get(acopy) _arraybola_2 (Variables|Default|GetArrayIndexStartDelete))))
                                        (Utilities|Array|RemoveIndex _arraybola_2 (Variables|Default|GetArrayIndexStartDelete))
                                        (Actor|DestroyActor _output_get_6)
                                        (CallFunction|ResetIndex)
                                        (CallFunction|MoveBackward self))
                                      (Variables|Default|Settarget (* (Variables|Default|Getcount) 30))
                                      (Variables|Default|Setcount 1)
                                      (goto _label Break)
                                      (else
                                        (Variables|Default|Setcount 1)
                                        (if (== (Variables|Default|GetArray%20Index) (- (Utilities|Array|LastIndex (Variables|Default|GetarrayBola)) 1))
                                          (Variables|Default|Setrepeat false)
                                          (goto _label Break)))))))
                              (:CastFailed
                                (Utilities|Casting|CastToBP_PurpleBall _array_element)
                                (Utilities|Casting|CastToBP_PurpleBall (Utilities|Array|Get(acopy) (Variables|Default|GetarrayBola) (+ (Variables|Default|GetArray%20Index) 1))
                                  (:then
                                    (bind _result_7 (Math|Integer|IncrementInt (Variables|Default|Getcount))
                                      (:%20%20
                                        (Variables|Default|Setcount _result_7))))
                                  (:CastFailed
                                    (if (>= (Variables|Default|Getcount) 3)
                                      (Variables|Default|SetArrayIndexStartDelete (- (Variables|Default|GetArray%20Index) (- (Variables|Default|Getcount) 1)))
                                      (for _index_7 (range 0 (- (Variables|Default|Getcount) 1))
                                        (bind _output_get_7 (Variables|Default|SetTempObject (Utilities|Array|Get(acopy) _arraybola_4 (Variables|Default|GetArrayIndexStartDelete))))
                                        (Utilities|Array|RemoveIndex _arraybola_4 (Variables|Default|GetArrayIndexStartDelete))
                                        (Actor|DestroyActor _output_get_7)
                                        (CallFunction|ResetIndex)
                                        (CallFunction|MoveBackward self))
                                      (Variables|Default|Settarget (* (Variables|Default|Getcount) 30))
                                      (Variables|Default|Setcount 1)
                                      (goto _label Break)
                                      (else
                                        (Variables|Default|Setcount 1)
                                        (if (== (Variables|Default|GetArray%20Index) (- (Utilities|Array|LastIndex (Variables|Default|GetarrayBola)) 1))
                                          (Variables|Default|Setrepeat false)
                                          (goto _label Break))))))))))))))))))))))

(event Custom|Move_Backward
  (for _index (range 0 (- (Variables|Default|GetArray%20Index) (Variables|Default|Getcount)))
    (Default|GetCount (Utilities|Array|Get(acopy) (Variables|Default|GetarrayBola) _index) (Variables|Default|Getcount) -1)))

(event EventBeginPlay
  (bind _road (Variables|Default|GetRoad))
  (Utilities|FlowControl|Sequence
    (:then_0
      (for _index (range 0 9)
        (bind _output_get (Variables|Default|Setrandom (Math|Random|RandomIntegerinRange 0 6)))
        (if (== _output_get 0)
          (bind _returnvalue (Game|SpawnActorfromClass "/Game/Blueprint/BP_RedBall.BP_RedBall_C" (Math|Transform|MakeTransform "-315.000000,690.000000,95.000000" "0, 0, 0" "1.000000,1.000000,1.000000") "Undefined" 0 _road _index true self 0))
          (Utilities|Array|Add (Variables|Default|GetarrayBola) _returnvalue)
          (Default|GetIndexFrame _returnvalue (/ (Spline|GetSplineLength (Variables|Default|GetRoad)) 3.6e+03))
          (elif (== _output_get 1)
            (bind _returnvalue_2 (Game|SpawnActorfromClass "/Game/Blueprint/BP_OrangeBall.BP_OrangeBall_C" (Math|Transform|MakeTransform "-315.000000,690.000000,95.000000" "0, 0, 0" "1.000000,1.000000,1.000000") "Undefined" 0 _road _index true self 0))
            (Utilities|Array|Add (Variables|Default|GetarrayBola) _returnvalue_2)
            (Default|GetIndexFrame _returnvalue_2 (/ (Spline|GetSplineLength (Variables|Default|GetRoad)) 3.6e+03))
            (elif (== _output_get 2)
              (bind _returnvalue_3 (Game|SpawnActorfromClass "/Game/Blueprint/BP_YellowBall.BP_YellowBall_C" (Math|Transform|MakeTransform "-315.000000,690.000000,95.000000" "0, 0, 0" "1.000000,1.000000,1.000000") "Undefined" 0 _road _index true self 0))
              (Utilities|Array|Add (Variables|Default|GetarrayBola) _returnvalue_3)
              (Default|GetIndexFrame _returnvalue_3 (/ (Spline|GetSplineLength (Variables|Default|GetRoad)) 3.6e+03))
              (elif (== _output_get 3)
                (bind _returnvalue_4 (Game|SpawnActorfromClass "/Game/Blueprint/BP_GreenBall.BP_GreenBall_C" (Math|Transform|MakeTransform "-315.000000,690.000000,95.000000" "0, 0, 0" "1.000000,1.000000,1.000000") "Undefined" 0 _road _index true self 0))
                (Utilities|Array|Add (Variables|Default|GetarrayBola) _returnvalue_4)
                (Default|GetIndexFrame _returnvalue_4 (/ (Spline|GetSplineLength (Variables|Default|GetRoad)) 3.6e+03))
                (elif (== _output_get 4)
                  (bind _returnvalue_5 (Game|SpawnActorfromClass "/Game/Blueprint/BP_BlueBall.BP_BlueBall_C" (Math|Transform|MakeTransform "-315.000000,690.000000,95.000000" "0, 0, 0" "1.000000,1.000000,1.000000") "Undefined" 0 _road _index true self 0))
                  (Utilities|Array|Add (Variables|Default|GetarrayBola) _returnvalue_5)
                  (Default|GetIndexFrame _returnvalue_5 (/ (Spline|GetSplineLength (Variables|Default|GetRoad)) 3.6e+03))
                  (elif (== _output_get 5)
                    (bind _returnvalue_6 (Game|SpawnActorfromClass "/Game/Blueprint/BP_PinkBall.BP_PinkBall_C" (Math|Transform|MakeTransform "-315.000000,690.000000,95.000000" "0, 0, 0" "1.000000,1.000000,1.000000") "Undefined" 0 _road _index true self 0))
                    (Utilities|Array|Add (Variables|Default|GetarrayBola) _returnvalue_6)
                    (Default|GetIndexFrame _returnvalue_6 (/ (Spline|GetSplineLength (Variables|Default|GetRoad)) 3.6e+03))
                    (else
                      (bind _returnvalue_7 (Game|SpawnActorfromClass "/Game/Blueprint/BP_PurpleBall.BP_PurpleBall_C" (Math|Transform|MakeTransform "-315.000000,690.000000,95.000000" "0, 0, 0" "1.000000,1.000000,1.000000") "Undefined" 0 _road _index true self 0))
                      (Utilities|Array|Add (Variables|Default|GetarrayBola) _returnvalue_7)
                      (Default|GetIndexFrame _returnvalue_7 (/ (Spline|GetSplineLength (Variables|Default|GetRoad)) 3.6e+03)))))))))))
    (:then_1
      (Utilities|Time|SetTimerbyFunctionName 0 "CheckCombo" 0.3 true))))

(fn ConstructionScript
  (bind _road (Variables|Default|GetRoad))
  (for _index (range 0 (- (Spline|GetNumberOfSplinePoints (Variables|Default|GetRoad)) 2))
    (bind _returnvalue (AddComponent|AddSplineMeshComponent false))
    (Components|StaticMesh|SetStaticMesh _returnvalue (Variables|Default|GetObjectSpline))
    (SplineMesh|SetStartandEnd _returnvalue (.Location (Spline|GetLocationandTangentatSplinePoint _road _index "Local")) (.Tangent (Spline|GetLocationandTangentatSplinePoint _road _index "Local")) (.Location (Spline|GetLocationandTangentatSplinePoint _road (+ _index 1) "Local")) (.Tangent (Spline|GetLocationandTangentatSplinePoint _road (+ _index 1) "Local")) true :!class /Script/Engine.SplineMeshComponent)
    (Transformation|AttachComponentToComponent _returnvalue (Variables|Default|GetDefaultSceneRoot) "None" "KeepRelative" "KeepRelative" "KeepRelative" true)))